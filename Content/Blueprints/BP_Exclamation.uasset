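; BP_Exclamation is the draw-signal actor for a samurai duel, registering with GM_Duel and prompting the player pawn to set its reference.
; StartDuel shows the exclamation immediately, then waits a random delay before ShowExlamation plays a yell and opens GM_Duel's CanAttack window.
; After a timed window, it hides the exclamation and clears that flag.
; Its own CanAttack, returned by IsAttackAllowed, is only ever set false here.
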(event `self.ReceiveBeginPlay`
  (bind _asgm_duel (cast `/Game/GameMode/GM_Duel` (`GameplayStatics.GetGameMode`)))
  (`/Game/GameMode/GM_Duel.RegExclmtn` _asgm_duel self)
  (bind _asbp_samurai_player (cast `/Game/Blueprints/BP_SamuraiPlayer` (`GameplayStatics.GetPlayerPawn` 0)))
  (`/Game/Blueprints/BP_SamuraiPlayer.SetExclamationReference` _asbp_samurai_player))

(event `StartDuel`
  ;[0.05551 1 1.6e-05] Start Duel Logic (To be called inside GM_Duel)
  (set `self.CanAttack` false)
  (`SceneComponent.SetVisibility` (`self.Exclamation`) true false)
  (`KismetSystemLibrary.Delay` (`KismetMathLibrary.RandomFloatInRange` (`self.DrawDelayMin`) (`self.DrawDelayMax`)))
  (`self.ShowExlamation`))

(event `ShowExlamation`
  ;[1 0 0.04439] Exclamation Visibility Logic
  (`SceneComponent.SetVisibility` (`self.Exclamation`) true false)
  (`KismetSystemLibrary.PrintString` "Exclamation Shown")
  (`GameplayStatics.PlaySound2D` "/Game/Audio/samurai_yell_Cue.samurai_yell_Cue" 1.0 1.0 0.0 null null)
  (bind _asgm_duel (cast `/Game/GameMode/GM_Duel` (`GameplayStatics.GetGameMode`)))
  (bind _output_get (set `/Game/GameMode/GM_Duel.CanAttack` true _asgm_duel))
  (`KismetSystemLibrary.PrintString` "Can Attack Yes" _output_get true (struct :`R` 1.0 :`B` 0.044391 :`A` 1.0) 2.0 "1")
  (`KismetSystemLibrary.Delay` (`self.AttackWIndowTime`))
  (`self.EndAttack`)
  (bind _asgm_duel_2 (cast `/Game/GameMode/GM_Duel` (`GameplayStatics.GetGameMode`)))
  (set `/Game/GameMode/GM_Duel.CanAttack` false _asgm_duel_2))

(event `EndAttack`
  ;[0.05551 1 1.6e-05] End Attack Logic
  (`SceneComponent.SetVisibility` (`self.Exclamation`) false false)
  (set `self.CanAttack` false))

(fn `IsAttackAllowed?`
  (returns (Allowed :type Boolean))
  (return (`self.CanAttack`)))

(fn `UserConstructionScript`)