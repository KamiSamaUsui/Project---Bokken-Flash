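; BP_SamuraiNPC is the enemy duelist, shown as a toad sprite, in a samurai duel game.
; On BeginPlay it registers itself with the GM_Duel game mode.
; Its EnemyAttack event, if the duel is not finished, switches the enemy to Attack and sets the BP_SamuraiPlayer state to Defeated.
; UpdateEnemyState swaps the sprite for the Idle, Attack and Defeated states.
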(event `self.ReceiveBeginPlay`
  (bind _asgm_duel (cast `/Game/GameMode/GM_Duel` (`GameplayStatics.GetGameMode`)))
  (`/Game/GameMode/GM_Duel.RegisterEnemy` _asgm_duel self))

(event `EnemyAttack`
  ;[0.05551 1 1.6e-05] Enemy Attack Logic
  (bind _asgm_duel (cast `/Game/GameMode/GM_Duel` (`GameplayStatics.GetGameMode`)))
  (if (not (`/Game/GameMode/GM_Duel.DuelFinished` _asgm_duel))
    (`self.UpdateEnemyState` "NewEnumerator1")
    (bind _asbp_samurai_player (cast `/Game/Blueprints/BP_SamuraiPlayer` (`GameplayStatics.GetPlayerCharacter` 0)))
    (`/Game/Blueprints/BP_SamuraiPlayer.Update Samurai State` _asbp_samurai_player "NewEnumerator2")))

(fn `UpdateEnemyState`
  (params (NewState :type "/Game/Blueprints/Enums/E_SamuraiStates Enum" :default "NewEnumerator0"))
  (bind _enemysprite (`self.EnemySprite`))
  (bind _output_get (set `self.New State` NewState))
  (switch `/Game/Blueprints/Enums/E_SamuraiStates` _output_get
    (:`NewEnumerator0`
      (`PaperSpriteComponent.SetSprite` _enemysprite "/Game/PaperAssets/Toad/T_Toad_Idle_Sprite.T_Toad_Idle_Sprite"))
    (:`NewEnumerator1`
      (`PaperSpriteComponent.SetSprite` _enemysprite "/Game/PaperAssets/Toad/T_Toad_Attack_Sprite.T_Toad_Attack_Sprite"))
    (:`NewEnumerator2`
      (`PaperSpriteComponent.SetSprite` _enemysprite "/Game/PaperAssets/Toad/T_Toad_Defeated_Sprite.T_Toad_Defeated_Sprite")))
  (return))

(fn `UserConstructionScript`)