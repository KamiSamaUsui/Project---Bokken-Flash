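; Game mode that runs a timed, samurai-style reaction duel, started shortly after play begins.
; StartDuel steps a phase enum through a random wait, an exclamation cue with a yell, an open attack window with a randomly delayed enemy attack, then closing.
; The exclamation and enemy are supplied through registration functions.
; IsAttackAllowed reports whether the duel is in the attack phase.
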(event `self.ReceiveBeginPlay`
  ;[0.05551 1 1.6e-05] EventBeginPlay
  (`KismetSystemLibrary.Delay` 5.0)
  (`self.StartDuel`))

(event `StartDuel`
  (bind _enemyref (`self.EnemyRef`))
  ;[0.05551 1 1.6e-05] Start Duel From Game Mode
  (set `self.DuelPhase` "NewEnumerator0")
  (`KismetSystemLibrary.Delay` (`KismetMathLibrary.RandomFloatInRange` 2.5 5.0))
  (`/Game/Blueprints/BP_Exclamation.ShowExlamation` (`self.ExclamationRef`))
  (set `self.DuelPhase` "NewEnumerator1")
  (`GameplayStatics.PlaySound2D` "/Game/Audio/samurai_yell_Cue.samurai_yell_Cue" 1.0 1.0 0.0 null null)
  (set `self.AttackWindowOpen` true)
  (set `self.DuelPhase` "NewEnumerator2")
  (`KismetSystemLibrary.Delay` (`KismetMathLibrary.RandomFloatInRange` 0.35 1.2))
  (set `self.EnemyRef` _enemyref)
  (`/Game/Blueprints/BP_SamuraiNPC.EnemyAttack` _enemyref)
  (`KismetSystemLibrary.Delay` 0.9)
  (set `self.AttackWindowOpen` false)
  (set `self.DuelPhase` "NewEnumerator3")
  (`/Game/Blueprints/BP_Exclamation.EndAttack` (`self.ExclamationRef`)))

(fn `IsAttackAllowed?`
  (returns (NewParam :type Boolean))
  (return (`|EnumEquality` (`self.DuelPhase`) "NewEnumerator2")))

(fn `RegExclmtn`
  (params (Exclamation :type "/Game/Blueprints/BP_Exclamation Object Reference"))
  (set `self.ExclamationRef` Exclamation)
  (`KismetSystemLibrary.PrintString` "EXCL REGISTERED")
  (return))

(fn `RegisterEnemy`
  (params (Enemy :type "/Game/Blueprints/BP_SamuraiNPC Object Reference"))
  (bind _output_get (set `self.EnemyRef` Enemy))
  (`KismetSystemLibrary.PrintString` (`KismetSystemLibrary.GetDisplayName` _output_get)))

(fn `UserConstructionScript`)